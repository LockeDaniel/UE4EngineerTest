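; BP_RobotGrabber is an AI robot Blueprint that refills its instruction queue with a sphere-search routine whenever that queue runs empty.
; On InstructionsAreEmpty, it queues alternating sphere checks and partial rotations, splitting a configurable sweep angle across a set number of turns.
; Each rotation follows the last wall rotation direction, and a fixed-distance forward move closes the routine.
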(event `self.InstructionsAreEmpty`
  (for _ (range (+ (`self.SphereCheckTurns`) 1))
    (`|ExecutionSequence`
      (:`then_0`
        (bind _returnvalue (`RInstructionCheckForSpheres.CreateInstructionCheckForSpheres`))
        (`self.AddInstruction` _returnvalue))
      (:`then_1`
        (bind _returnvalue_2 (`self.GetLastWallRotationDirection`))
        (bind _returnvalue_3 (`RInstructionRotate.CreateInstructionRotate` (* _returnvalue_2 (/ (`self.SphereCheckRotation`) (`KismetMathLibrary.Conv_IntToDouble` (`self.SphereCheckTurns`))))))
        (`self.AddInstruction` _returnvalue_3))))
  (bind _returnvalue_4 (`RInstructionMoveForward.CreateInstructionMoveForward` 750.0))
  (`self.AddInstruction` _returnvalue_4))

(fn `UserConstructionScript`)